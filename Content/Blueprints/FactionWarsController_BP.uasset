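; Player controller for Faction Wars that handles targeting and ability input for the controlled FactionWarsCharacter.
; Left-clicks off widgets and hostile/ally cycle keys, which wrap through the character's target arrays, feed SetControllerTarget, which updates the target and switches selection decals.
; Eight ability keys and AbilityClickedBP resolve a slot index for UseThisAbility, which is defined outside this file.
; The ToggleSpellBook input only casts the game mode and is marked as an error.
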(event Custom|AbilityClickedBP
  (params (AbilityContainer :type Active%20Ability%20Container%20Object%20Reference))
  (bind _chararef (Variables|Default|GetCharaRef))
  (bind _abilitycontainersarray (Variables|/Script/FactionWars.FactionWarsCharacter|GetAbilityContainersArray _chararef))
  (bind _returnvalue (Utilities|Array|FindItem _abilitycontainersarray AbilityContainer))
  (if (Utilities|Array|IsValidIndex _abilitycontainersarray _returnvalue)
    (Class|PlayerControllerFW|UseThisAbility _returnvalue)))

(event EventBeginPlay
  (|CallParentFunction)
  (bind _asfaction_wars_character_bp (Utilities|Casting|CastToFactionWarsCharacter_BP (Pawn|GetControlledPawn)))
  (Variables|Default|SetCharaRef _asfaction_wars_character_bp))

(event EventTick
  (params (DeltaSeconds :type Float%20%28single-precision%29))
  (|CallParentFunction DeltaSeconds))

(event Input|ActionEvents|InputActionUseAbility1
  (params (Key :type Key%20Structure :default "None"))
  (:Pressed
    (Class|PlayerControllerFW|UseThisAbility)))

(event Input|ActionEvents|InputActionUseAbility2
  (params (Key :type Key%20Structure :default "None"))
  (:Pressed
    (Class|PlayerControllerFW|UseThisAbility 1)))

(event Input|ActionEvents|InputActionCycleHostileTarget
  (params (Key :type Key%20Structure :default "None"))
  (:Pressed
    (bind _chararef (Variables|Default|GetCharaRef)
      (:then
        (CallFunction|CycleTarget _chararef (Variables|/Script/FactionWars.FactionWarsCharacter|GetPossibleHostileTargets _chararef)))
      (:else))))

(event Input|ActionEvents|InputActionCycleAllyTarget
  (params (Key :type Key%20Structure :default "None"))
  (:Pressed
    (bind _chararef (Variables|Default|GetCharaRef)
      (:then
        (CallFunction|CycleTarget _chararef (Variables|/Script/FactionWars.FactionWarsCharacter|GetPossibleAllyTargets _chararef)))
      (:else))))

(event Input|ActionEvents|InputActionUseAbility3
  (params (Key :type Key%20Structure :default "None"))
  (:Pressed
    (Class|PlayerControllerFW|UseThisAbility 2)))

(event Input|ActionEvents|InputActionUseAbility4
  (params (Key :type Key%20Structure :default "None"))
  (:Pressed
    (Class|PlayerControllerFW|UseThisAbility 3)))

(event Input|ActionEvents|InputActionUseAbility5
  (params (Key :type Key%20Structure :default "None"))
  (:Pressed
    (Class|PlayerControllerFW|UseThisAbility 4)))

(event Input|ActionEvents|InputActionUseAbility6
  (params (Key :type Key%20Structure :default "None"))
  (:Pressed
    (Class|PlayerControllerFW|UseThisAbility 5)))

(event Input|ActionEvents|InputActionUseAbility7
  (params (Key :type Key%20Structure :default "None"))
  (:Pressed
    (Class|PlayerControllerFW|UseThisAbility 6)))

(event Input|ActionEvents|InputActionUseAbility8
  (params (Key :type Key%20Structure :default "None"))
  (:Pressed
    (Class|PlayerControllerFW|UseThisAbility 7)))

(event Input|ActionEvents|InputActionToggleSpellBook
  (params (Key :type Key%20Structure :default "None"))
  (:Pressed
    ;[1 1 1] error
    (bind _asfaction_wars_game_mode_bp (Utilities|Casting|CastToFactionWarsGameMode_BP (Game|GetGameMode)))))

(event Input|MouseEvents|LeftMouseButton
  (params (Key :type Key%20Structure :default "None"))
  (:Pressed
    (if (not (Variables|Default|GetIsMouseOnWidget))
      (CallFunction|SetControllerTarget (.HitActor (Collision|BreakHitResult (.HitResult (Game|Player|GetHitResultUnderCursorbyChannel "TraceTypeQuery1" true))))))))

(fn ConstructionScript)

(fn InvalidateTarget
  (bind _returnvalue (Class|FactionWarsCharacter|GetTarget (Variables|Default|GetCharaRef)))
  (bind _asfaction_wars_character_bp (Utilities|Casting|CastToFactionWarsCharacter_BP _returnvalue))
  (Default|SwitchDecalVisibility _asfaction_wars_character_bp)
  (Class|FactionWarsCharacter|SetTarget (Variables|Default|GetCharaRef)))

(fn SetMouseonWidget
  (params (Input :type Pointer%20Event%20Structure%20%28by%20ref%29) (IsMouseOnWidget :type Boolean))
  (if (not (Class|KismetInputLibrary|PointerEventIsMouseButtonDown Input "LeftMouseButton"))
    (Variables|Default|SetIsMouseOnWidget IsMouseOnWidget)))

(fn SetControllerTarget
  (params (Actor :type Object%20Object%20Reference))
  (bind _chararef (Variables|Default|GetCharaRef))
  (bind _asfaction_wars_character_bp (Utilities|Casting|CastToFactionWarsCharacter_BP Actor)
    (:then
      (bind _returnvalue (Class|FactionWarsCharacter|GetTarget (Variables|Default|GetCharaRef)))
      (bind _asfaction_wars_character_bp_2 (Utilities|Casting|CastToFactionWarsCharacter_BP _returnvalue)
        (:then
          (if (!= _asfaction_wars_character_bp_2 _asfaction_wars_character_bp)
            (CallFunction|InvalidateTarget :!label _label)
            (Class|FactionWarsCharacter|SetTarget _chararef _asfaction_wars_character_bp)
            (Default|SwitchDecalVisibility _asfaction_wars_character_bp _chararef)))
        (:CastFailed
          (if (== _asfaction_wars_character_bp_2 0)
            (goto _label)))))
    (:CastFailed
      (CallFunction|InvalidateTarget))))

(fn CycleTarget
  (params (CharaRef :type Faction%20Wars%20Character%20Object%20Reference) (TargetArray :type Array%20of%20Faction%20Wars%20Character%20Object%20References))
  (bind _output (Utilities|Array|Get(acopy) TargetArray))
  (bind _returnvalue (Class|FactionWarsCharacter|GetTarget CharaRef))
  (Utilities|IsValid _returnvalue
    (:Is%20Valid
      (if (Utilities|Array|IsValidIndex TargetArray (Utilities|Array|FindItem TargetArray _returnvalue))
        (Utilities|IsValid (Utilities|Array|Get(acopy) TargetArray (Math|Integer|%(Integer) (+ (Utilities|Array|FindItem TargetArray _returnvalue) 1) (Utilities|Array|Length TargetArray)))
          (:Is%20Valid
            (CallFunction|SetControllerTarget (Utilities|Array|Get(acopy) TargetArray (Math|Integer|%(Integer) (+ (Utilities|Array|FindItem TargetArray _returnvalue) 1) (Utilities|Array|Length TargetArray))))))
        (else
          (Utilities|IsValid _output :!label _label
            (:Is%20Valid
              (CallFunction|SetControllerTarget _output))))))
    (:Is%20Not%20Valid
      (goto _label))))