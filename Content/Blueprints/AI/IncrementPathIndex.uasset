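; Behavior Tree task that advances an AI character's patrol to the next point on its assigned path.
; On execute it casts the pawn to FactionWarsCharacter_BP and reads its PatrolPath points.
; It increments the PatrolPathIndex blackboard key, wrapping with modulo so the patrol loops, and finishes successfully.
; It fails if the cast, path or resulting index is invalid.
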(event EventReceiveExecuteAI
  (params (OwnerController :type AI%20Controller%20Object%20Reference) (ControlledPawn :type Pawn%20Object%20Reference))
  (bind _asfaction_wars_character_bp (Utilities|Casting|CastToFactionWarsCharacter_BP ControlledPawn)
    (:then
      (bind _patrolpath (Variables|/Game/Blueprints/Characters/FactionWarsCharacter_BP.FactionWarsCharacter_BP_C|GetPatrolPath _asfaction_wars_character_bp)
        (:then
          (if (Utilities|Array|IsValidIndex (Variables|/Game/Blueprints/AI/PatrolPath.PatrolPath_C|GetPathPoints _patrolpath) (Math|Integer|%(Integer) (+ (Class|BTFunctionLibrary|GetBlackboardValueasInt (Variables|Default|GetPatrolPathIndex)) 1) (Utilities|Array|Length (Variables|/Game/Blueprints/AI/PatrolPath.PatrolPath_C|GetPathPoints _patrolpath))))
            (Class|BTFunctionLibrary|SetBlackboardValueasInt (Variables|Default|GetPatrolPathIndex) (Math|Integer|%(Integer) (+ (Class|BTFunctionLibrary|GetBlackboardValueasInt (Variables|Default|GetPatrolPathIndex)) 1) (Utilities|Array|Length (Variables|/Game/Blueprints/AI/PatrolPath.PatrolPath_C|GetPathPoints _patrolpath))))
            (AI|BehaviorTree|FinishExecute true)
            (else
              (AI|BehaviorTree|FinishExecute false :!label _label))))
        (:else
          (goto _label))))
    (:CastFailed
      (goto _label))))