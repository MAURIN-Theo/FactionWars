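; GameState Blueprint that sets up the player's HUD and mouse input when play begins.
; BeginPlay creates a HeadsUpDisplay_New widget for player controller 0, stores it in HUDwidget and adds it to the viewport.
; It then switches that controller to Game and UI input mode and shows the mouse cursor, with each step guarded by a validity check.
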(event EventBeginPlay
  (CallFunction|CreateandAddHUD)
  (CallFunction|EnableMouseCursor))

(event EventTick
  (params (DeltaSeconds :type Float%20%28single-precision%29)))

(fn ConstructionScript)

(fn CreateandAddHUD
  (bind _returnvalue (Game|GetPlayerController 0))
  (Utilities|IsValid _returnvalue
    (:Is%20Valid
      (bind _returnvalue_2 (UserInterface|CreateWidget "/Game/AbilitySystem/UI/HeadsUpDisplay_New.HeadsUpDisplay_New_C" _returnvalue))
      (bind _output_get (Variables|Default|SetHUDwidget _returnvalue_2))
      (UserInterface|Viewport|AddtoViewport _output_get 0))))

(fn EnableMouseCursor
  (bind _returnvalue (Game|GetPlayerController 0))
  (Utilities|IsValid _returnvalue
    (:Is%20Valid
      (Input|SetInputModeGameandUI _returnvalue 0 "DoNotLock" true)
      (Variables|/Script/Engine.PlayerController|SetbShowMouseCursor _returnvalue true))))