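; Quadruped character Blueprint from the Animal Variety Pack that turns movement axis input into animal locomotion.
; MoveForward accepts only forward input along MoveRotTarget, whose yaw eases toward the control rotation for gradual turning.
; MoveRight blends that target's right vector with the actor's facing, so sideways input produces diagonal forward movement.
; A wolf jump-bite montage with speed-based section selection is present but unconnected.
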(event EventBeginPlay
  (|CallParentFunction) ; This node is disabled and will not be called.\nDrag off pins to build functionality.
)

(event Collision|EventActorBeginOverlap
  (params (OtherActor :type Actor%20Object%20Reference)))

(event EventTick
  (params (DeltaSeconds :type Float%20%28single-precision%29))
  (|CallParentFunction DeltaSeconds) ; This node is disabled and will not be called.\nDrag off pins to build functionality.
)

(event EventMoveRight
  (params (Value :type Float%20%28single-precision%29))
  (Pawn|Input|AddMovementInput (Math|Vector|Normalize (+ (* (Math|Vector|GetRightVector (Variables|Default|GetMoveRotTarget)) Value) (Math|Vector|GetForwardVector (Math|Rotator|MakeRotator 0.0 0.0 (.yaw (Transformation|GetActorRotation)))))) (Math|Float|Absolute(Float) Value) false))

(event EventMoveForward
  (params (Value :type Float%20%28single-precision%29))
  (Pawn|Input|AddMovementInput (Math|Vector|GetForwardVector (Variables|Default|GetMoveRotTarget)) (Math|Float|Clamp(Float) Value) false)
  (Variables|Default|SetMoveRotTarget (Math|Rotator|MakeRotator 0.0 0.0 (.yaw (Math|Interpolation|RInterpTo (Variables|Default|GetMoveRotTarget) (Pawn|GetControlRotation :!class /Script/Engine.Pawn) (Utilities|Time|GetWorldDeltaSeconds) 3.0)))))

(event Input|ActionEvents|InputActionJump
  (params (Key :type Key%20Structure :default "None")))

(fn ConstructionScript
  (|CallParentFunction))