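; Base ability actor for Faction Wars, with mostly empty or unwired cast logic.
; BeginCasting calls CastAbility directly when CastTime is not positive; its cast-bar binding is disconnected, as is the event graph's call to BeginCasting.
; InterruptCast destroys the actor and calls CastInterrupted, while AttachToSocket snaps to the caster's right-hand socket.
; GetControllerRef caches the player controller; GetHUD contains an error and GetPlayerRef is unwired.
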(event Custom|CastAbility)

(event EventBeginPlay)

(event Collision|EventActorBeginOverlap
  (params (OtherActor :type Actor%20Object%20Reference)))

(event EventTick
  (params (DeltaSeconds :type Float%20%28single-precision%29)))

(fn ConstructionScript)

(fn BeginCasting
  (if (not (> (.casttime (Variables|Default|GetAbilityDetails)) 0.0))
    (CallFunction|CastAbility)))

(fn GetHUD
  ;[1 1 1] error
  (bind _asfaction_wars_game_mode_bp (Utilities|Casting|CastToFactionWarsGameMode_BP (Game|GetGameMode)))
  (Variables|Default|SetHUDwidget 0)
  (return))

(fn InterruptCast
  (Actor|DestroyActor)
  (Default|CallCastInterrupted))

(fn ActivateEffect)

(fn GetPlayerRef)

(fn AttachtoSocket
  (Transformation|AttachComponentToComponent (Variables|/Script/Engine.Character|GetMesh (Variables|Default|GetCaster)) "hand_rSocket" "SnapToTarget" "SnapToTarget" "SnapToTarget" true))

(fn GetControllerRef
  (bind _asfaction_wars_controller_bp (Utilities|Casting|CastToFactionWarsController_BP (Game|GetPlayerController 0)))
  (Variables|Default|SetController _asfaction_wars_controller_bp)
  (return))